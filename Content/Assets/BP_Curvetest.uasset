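; BP_Curvetest is an unfinished test actor that appears intended to guide the physics ball's camera along a track.
; It caches the player's PhysicsBallBP pawn on BeginPlay, and Curve_coll overlaps with the ball toggle ActiveTrack.
; Tick checks that flag but does nothing.
; Disconnected nodes sketch moving the ball's MainCamera and interpolating toward the closest point on the Track spline.
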(event OnComponentBeginOverlap(curve_coll)
  (params (OverlappedComponent :type Primitive%20Component%20Object%20Reference) (OtherActor :type Actor%20Object%20Reference) (OtherComp :type Primitive%20Component%20Object%20Reference) (OtherBodyIndex :type Integer) (bFromSweep :type Boolean) (SweepResult :type Hit%20Result%20Structure%20%28by%20ref%29))
  (Utilities|Casting|CastToPhysicsBallBP OtherActor)
  (Variables|Default|SetActiveTrack true))

(event OnComponentEndOverlap(curve_coll)
  (params (OverlappedComponent :type Primitive%20Component%20Object%20Reference) (OtherActor :type Actor%20Object%20Reference) (OtherComp :type Primitive%20Component%20Object%20Reference) (OtherBodyIndex :type Integer))
  (Utilities|Casting|CastToPhysicsBallBP OtherActor)
  (Variables|Default|SetActiveTrack false))

(event EventBeginPlay
  (bind _asphysics_ball_bp (Utilities|Casting|CastToPhysicsBallBP (Game|Player|GetPlayerPawn 0)))
  (Variables|Default|SetRollBall _asphysics_ball_bp))

(event Collision|EventActorBeginOverlap
  (params (OtherActor :type Actor%20Object%20Reference)))

(event EventTick
  (params (DeltaSeconds :type Float%20%28single-precision%29))
  (if (Variables|Default|GetActiveTrack)
    _))

(fn ConstructionScript)