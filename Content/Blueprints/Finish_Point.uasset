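; Finish line actor for a rolling-ball race that ends the run when a PhysicsBallBP overlaps it.
; On overlap it sets IsFirst, shows the Race_Complete widget, and tells RollingGameMode to begin flashing and stop the timer.
; After a short delay it removes all widgets, opens the Menu_Finish screen and shows the mouse cursor.
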(event Collision|EventActorBeginOverlap
  (params (OtherActor :type Actor%20Object%20Reference))
  (Utilities|Casting|CastToPhysicsBallBP OtherActor)
  (Variables|Default|SetIsFirst true)
  (Development|PrintString "Race Complete")
  (bind _returnvalue (UserInterface|CreateWidget "/Game/Widgets/Race_Complete.Race_Complete_C"))
  (UserInterface|Viewport|AddtoPlayerScreen _returnvalue)
  (bind _asrolling_game_mode (Utilities|Casting|CastToRollingGameMode (Game|GetGameMode)))
  (Default|BeginFlashing _asrolling_game_mode)
  (Variables|/Game/Blueprints/RollingGameMode.RollingGameMode_C|SetRunTimer _asrolling_game_mode false)
  (Utilities|FlowControl|Delay 5.0)
  (Viewport|RemoveAllWidgets)
  (bind _returnvalue_2 (UserInterface|CreateWidget "/Game/Widgets/Menu_Finish.Menu_Finish_C"))
  (UserInterface|Viewport|AddtoViewport _returnvalue_2 0)
  (Variables|/Script/Engine.PlayerController|SetbShowMouseCursor (Game|GetPlayerController 0) true))

(fn ConstructionScript)