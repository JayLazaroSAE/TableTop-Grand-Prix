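; PositionZone is a trigger actor that works out the player's arrival position, apparently for placing in a ball game.
; While its Count flag is set, each begin-overlap from any actor increments a Position counter.
; When player 0's pawn overlaps, it prints the position, clears Count to freeze the tally, and writes Position to BallPlayerController.
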(event Collision|EventActorBeginOverlap
  (params (OtherActor :type Actor%20Object%20Reference))
  (if (Variables|Default|GetCount)
    (bind _result (Math|Integer|IncrementInt (Variables|Default|GetPosition))
      (:%20%20
        (bind _output_get (Variables|Default|SetPositionString (Utilities|String|ToString(Integer) _result)))
        (if (== OtherActor (Game|Player|GetPlayerPawn 0))
          (Development|PrintString _output_get)
          (Variables|Default|SetCount false)
          (bind _asball_player_controller (Utilities|Casting|CastToBallPlayerController (Game|GetPlayerController 0)))
          (Variables|/Game/Blueprints/BallPlayerController.BallPlayerController_C|SetPosition _asball_player_controller (Variables|Default|GetPosition)))))))

(fn ConstructionScript)