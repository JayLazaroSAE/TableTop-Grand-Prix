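; RollingGameMode is a game mode that shows the race UI on BeginPlay and keeps a race timer.
; While RunTimer is true, a one-second Delay on Tick counts up TimeSec and rolls it over into TimeMin.
; StartTimer waits five seconds, then creates and displays the Time widget.
; BeginFlashing uses a timeline to lerp that widget's timer color between opaque and transparent white.
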(event Custom|Begin%20Flashing
  (bind _alpha (Timeline|Timeline_0 Play)
    (:Update
      (Variables|/Game/Widgets/Time.Time_C|SetTimer%20Color (Variables|Default|GetTime%20Widget) (Utilities|Struct|MakeSlateColor (Math|Color|Lerp(LinearColor) "(R=1.000000,G=1.000000,B=1.000000,A=1.000000)" "(R=1.000000,G=1.000000,B=1.000000,A=0.000000)" _alpha))))))

(event Custom|Start%20Timer
  (Utilities|FlowControl|Delay 5.0)
  (bind _returnvalue (UserInterface|CreateWidget "/Game/Widgets/Time.Time_C"))
  (Variables|Default|SetTime%20Widget _returnvalue)
  (UserInterface|Viewport|AddtoViewport _returnvalue 0))

(event EventBeginPlay
  ;[1 1 1] Timer on UI
  (bind _returnvalue (UserInterface|CreateWidget "/Game/Widgets/RaceUI.RaceUI_C"))
  (UserInterface|Viewport|AddtoViewport _returnvalue 0))

(event EventTick
  (params (DeltaSeconds :type Float%20%28single-precision%29))
  ;[1 1 1] Timer on UI
  (Utilities|FlowControl|Delay 1.0) ; This delay adds 1 to the second digit
  (if (Variables|Default|GetRunTimer)
    (Variables|Default|SetTimeSec (+ (Variables|Default|GetTimeSec) 1))
    (if (> (Variables|Default|GetTimeSec) 59)
      (Variables|Default|SetTimeMin (+ (Variables|Default|GetTimeMin) 1))
      (Variables|Default|SetTimeSec 0))))

(fn ConstructionScript)