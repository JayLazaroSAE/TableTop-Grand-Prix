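; Finish line actor that ends the race when a PhysicsBallBP overlaps it.
; On overlap it sets IsFirst, prints a completion message and shows the Race_Complete widget on the player screen.
; After a short delay it removes all widgets, opens the Menu_Finish widget and shows the mouse cursor.
; IsFirst is never checked here, and the UI-only input mode node is left unconnected.
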(event EventBeginPlay)

(event EventTick
  (params (DeltaSeconds :type Float%20%28single-precision%29)))

(event Collision|EventActorBeginOverlap
  (params (OtherActor :type Actor%20Object%20Reference))
  (Utilities|Casting|CastToPhysicsBallBP OtherActor)
  (Variables|Default|SetIsFirst true)
  (Development|PrintString "Race Complete")
  (bind _returnvalue (UserInterface|CreateWidget "/Game/Widgets/Race_Complete.Race_Complete_C"))
  (UserInterface|Viewport|AddtoPlayerScreen _returnvalue)
  (Utilities|FlowControl|Delay 5.0)
  (Viewport|RemoveAllWidgets)
  (bind _returnvalue_2 (UserInterface|CreateWidget "/Game/Widgets/Menu_Finish.Menu_Finish_C"))
  (UserInterface|Viewport|AddtoViewport _returnvalue_2 0)
  (Variables|/Script/Engine.PlayerController|SetbShowMouseCursor (Game|GetPlayerController 0) true))

(fn ConstructionScript)