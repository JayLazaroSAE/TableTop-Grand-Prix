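; Game mode that puts a race UI on screen and keeps an elapsed-time clock in minutes and seconds.
; BeginPlay creates the RaceUI widget and adds it to the viewport.
; Tick runs a one-second Delay, which ignores re-triggers while pending, to increment TimeSec and roll it over into TimeMin after 59.
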(event EventBeginPlay
  ;[1 1 1] Timer on UI
  (bind _returnvalue (UserInterface|CreateWidget "/Game/Widgets/RaceUI.RaceUI_C"))
  (UserInterface|Viewport|AddtoViewport _returnvalue 0))

(event EventTick
  (params (DeltaSeconds :type Float%20%28single-precision%29))
  ;[1 1 1] Timer on UI
  (Utilities|FlowControl|Delay 1.0) ; This delay adds 1 to the second digit
  (Variables|Default|SetTimeSec (+ (Variables|Default|GetTimeSec) 1))
  (if (> (Variables|Default|GetTimeSec) 59)
    (Variables|Default|SetTimeMin (+ (Variables|Default|GetTimeMin) 1))
    (Variables|Default|SetTimeSec 0)))

(fn ConstructionScript)